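; Player spaceship character for the Asteroids game, handling input, shooting and the score and game-over UI.
; Axis inputs feed forward movement and yaw rotation functions defined outside these graphs.
; Holding Shoot sets a flag that Tick polls, firing BPShootComponent from left and right muzzle points, throttled by a DoOnce reset after a delay.
; BeginPlay shows the score widget; player death stops shooting and swaps that widget for the game-over screen.
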(event `self.OnPlayerDied`
  ;[1 0.4026 0.8802] Create Game over widget
  (set `self.bCanStartShooting` false)
  (bind _scorewidget (`self.ScoreWidget`)
    (:`then`
      (`Widget.RemoveFromParent` _scorewidget)
      (bind _returnvalue (`|CreateWidget` "/Game/Asteroids/UI/WBP_GameOver.WBP_GameOver_C"))
      (`UserWidget.AddToViewport` _returnvalue 0))
    (:`else`)))

(event `self.ReceiveBeginPlay`
  ;[0.4432 0.4348 1] Create Player widget
  (bind _returnvalue (`|CreateWidget` "/Game/Asteroids/UI/WBP_Score.WBP_Score_C"))
  (bind _output_get (set `self.ScoreWidget` _returnvalue))
  (`UserWidget.AddToViewport` _output_get 0))

(event `self.ReceiveTick`
  (params (DeltaSeconds :type "Float (single-precision)"))
  ;[0 0 0] Handle Shoot
  (if (`self.bCanStartShooting`)
    (`/Engine/EditorBlueprintResources/StandardMacros.DoOnce` false :!label _label
      (:`Completed`
        (`ShootComponent.Shoot` (`self.BP_ShootComponent`) (`|MakeArray` (`SceneComponent.K2_GetComponentLocation` (`self.ShootStartRight`)) (`SceneComponent.K2_GetComponentLocation` (`self.ShootStartLeft`))) (`SceneComponent.K2_GetComponentRotation` (`self.CapsuleComponent`)))
        (`KismetSystemLibrary.Delay` 0.3)
        (goto _label :!via `Reset`)))))

(event `InputAxis|MoveForward`
  (params (AxisValue :type "Float (single-precision)"))
  ;[1 0.5804 0.3462] Handle Inputs
  (`self.MoveForwardCharacter` AxisValue))

(event `InputAxis|RotateRight`
  (params (AxisValue :type "Float (single-precision)"))
  ;[1 0.5804 0.3462] Handle Inputs
  (`self.YawRotationCharacter` AxisValue))

(event `InputAction|Shoot`
  (params (Key :type "Key Structure"))
  ;[1 0.5804 0.3462] Handle Inputs
  (:`Pressed`
    (set `self.bCanStartShooting` true))
  (:`Released`
    (set `self.bCanStartShooting` false)))

(fn `UserConstructionScript`)